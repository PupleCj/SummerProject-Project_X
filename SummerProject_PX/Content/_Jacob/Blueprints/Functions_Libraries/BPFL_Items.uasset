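; BPFL_Items is a Blueprint function library for reading item definitions from the DB_Items data table.
; GetItemInfoFromDB looks up a row by ItemID and returns a success flag with the item info.
; GetRandomItemFromDB picks a random row name and returns success, ID and info.
; Its random index is re-evaluated for the returned ID, so ID and info can come from different rows.
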(fn GetItemInfofromDB
  (params (Item_ID :type Name))
  (bind _returnvalue (Utilities|GetDataTableRow "/Game/_Jacob/Blueprints/Data/Items/DB_Items.DB_Items" Item_ID)
    (:then
      (return true _returnvalue))
    (:RowNotFound
      (return false ""))))

(fn GetRandomItemfromDB
  (bind _outrownames (DataTable|GetDataTableRowNames "/Game/_Jacob/Blueprints/Data/Items/DB_Items.DB_Items"))
  (bind _returnvalue (Utilities|GetDataTableRow "/Game/_Jacob/Blueprints/Data/Items/DB_Items.DB_Items" (Utilities|Array|Get(acopy) _outrownames (Math|Random|RandomIntegerinRange 0 (- (Utilities|Array|Length _outrownames) 1))))
    (:then
      (return true (Utilities|Array|Get(acopy) _outrownames (Math|Random|RandomIntegerinRange 0 (- (Utilities|Array|Length _outrownames) 1))) _returnvalue))
    (:RowNotFound
      (return false "None" ""))))