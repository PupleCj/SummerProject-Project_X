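; Slot-based inventory component for player and loot inventories, which registers player inventories with the HUD and fills loot ones with random, optionally unique, database items.
; AddItem places items one at a time, stacking up to the database's max size before using empty slots, and returns the count added.
; Dropping async-loads the slot's actor class, decrements the slot, refreshes the HUD and spawns actors at the owner's drop position on a staggered delay.
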(event Custom|Drop_Items
  (params (Slot_Index :type Integer) (Amount_To_Drop :type Integer))
  ;[1 1 1] Drop Items
  (bind _class (Utilities|AsyncLoadClassAsset (.actor_class (Utilities|Array|Get(acopy) (Variables|Inventory|GetContent) Slot_Index)))
    (:Completed
      (bind _asactor (Utilities|Casting|CastToActorClass _class))
      (Variables|Helper|SetItem_To_Spawn _asactor)
      (CallFunction|DecrementSlotAmount Slot_Index Amount_To_Drop)
      (Utilities|ForLoopDelay 1 Amount_To_Drop 0.2
        (:Loop_Body
          (CallFunction|SpawnDroppedItems))))))

(event EventBeginPlay
  (CallFunction|InitializeInventory))

(fn InitializeInventory
  (for _index (range 1 (Variables|Inventory|GetSlots_Count))
    (Utilities|Array|Add (Variables|Inventory|GetContent) (Utilities|Struct|MakeStruct_Inventory_Slot "None" 0 false)))
  (switch Utilities|FlowControl|Switch|SwitchonEnum_Inventory_Types (Variables|Inventory|GetInventory_Type)
    (:NewEnumerator0
      (Class|BPIHUD|SetMainPlayerInventory(Message) (HUD|GetHUD (Game|GetPlayerController 0)) self))
    (:NewEnumerator2
      (CallFunction|AddRandomLoot))))

(fn FindEmptySlot
  (for (_array_element _array_index) (Variables|Inventory|GetContent)
    (if (not (.Occupied? (Utilities|Struct|BreakStruct_Inventory_Slot _array_element)))
      (return true _array_index)))
  (return false -1))

(fn FindAvailableSlotwithItem
  (params (Item_ID_to_Add :type Name))
  (bind (_success_ _item_info) (CallFunction|GetItemInfofromDB Item_ID_to_Add))
  (if _success_
    (for (_array_element _array_index) (Variables|Inventory|GetContent)
      (if (== Item_ID_to_Add (.Item_ID (Utilities|Struct|BreakStruct_Inventory_Slot _array_element)))
        (if (<= (+ (.Amount (Utilities|Struct|BreakStruct_Inventory_Slot _array_element)) 1) (.Max_Stack_Size (Utilities|Struct|BreakStruct_Items _item_info)))
          (return true _array_index))))
    (return false -1)))

(fn AddItemtoEmptySlot
  (params (Slot_Index :type Integer) (Item_ID_To_Add :type Name) (Actor_Class_To_Add :type Actor%20Soft%20Class%20Reference))
  (Utilities|Array|SetArrayElem (Variables|Inventory|GetContent) Slot_Index (Utilities|Struct|MakeStruct_Inventory_Slot Item_ID_To_Add 1 true Actor_Class_To_Add))
  (return true))

(fn AddItemtoSlotStack
  (params (Slot_Index :type Integer))
  (bind _content (Variables|Inventory|GetContent))
  (bind _output (Utilities|Array|Get(acopy) _content Slot_Index))
  (bind (_item_id _amount _occupied_ _actor_class) (Utilities|Struct|BreakStruct_Inventory_Slot _output))
  (Utilities|Array|SetArrayElem (Variables|Inventory|GetContent) Slot_Index (Utilities|Struct|MakeStruct_Inventory_Slot _item_id (+ _amount 1) _occupied_ _actor_class))
  (return true))

(fn AddItem
  (params (Item_ID_To_Add :type Name) (Amount_To_Add :type Integer))
  (bind (_success_ _item_info) (CallFunction|GetItemInfofromDB Item_ID_To_Add))
  ;[1 1 1] Setting the initial values
  (LocalVariables|SetItems_Left Amount_To_Add)
  (if _success_
    (LocalVariables|SetItem_Info _item_info)
    (for _index (range 1 Amount_To_Add)
      ;[1 1 1] If the item is stackable or not
      (if (.stackable? (LocalVariables|GetItem_Info))
        ;[1 1 1] Finding a slot with the item
        (bind (_success__2 _slot_index) (Helper|FindAvailableSlotwithItem Item_ID_To_Add))
        (if _success__2
          ;[1 1 1] Adding item to the same slot
          (bind _success__3 (Helper|AddItemtoSlotStack _slot_index))
          (if _success__3
            (LocalVariables|SetItems_Left (- (LocalVariables|GetItems_Left) 1)))
          (else
            ;[1 1 1] Adding item to an empty slot incase we didnt find a slot with the same item or if its already full
            (bind (_success__4 _slot_index_2) (Helper|FindEmptySlot))
            (if _success__4
              (bind _success__5 (Helper|AddItemtoEmptySlot _slot_index_2 Item_ID_To_Add (.actor_class (LocalVariables|GetItem_Info))))
              (if _success__5
                (LocalVariables|SetItems_Left (- (LocalVariables|GetItems_Left) 1)))
              (else
                (Development|PrintString "Inventory Full")))))
        (else
          ;[1 1 1] Finding an empty slot
          (bind (_success__6 _slot_index_3) (Helper|FindEmptySlot))
          (if _success__6
            ;[1 1 1] Adding item to an empty slot if the item is not stackable
            (bind _success__7 (Helper|AddItemtoEmptySlot _slot_index_3 Item_ID_To_Add (.actor_class (LocalVariables|GetItem_Info))))
            (if _success__7
              (LocalVariables|SetItems_Left (- (LocalVariables|GetItems_Left) 1)))
            (else
              (Development|PrintString "Inventory Full"))))))
    ;[1 1 1] Return the amount of items added
    (return (- Amount_To_Add (LocalVariables|GetItems_Left)))))

(fn DecrementSlotAmount
  (params (Slot_Index :type Integer) (Amount_To_Decrement :type Integer))
  (bind _content (Variables|Inventory|GetContent))
  (bind _output (Utilities|Array|Get(acopy) _content Slot_Index))
  (bind _returnvalue (- (.amount _output) Amount_To_Decrement))
  (if (<= _returnvalue 0)
    (Utilities|Array|SetArrayElem (Variables|Inventory|GetContent) Slot_Index (Utilities|Struct|MakeStruct_Inventory_Slot "None" 0 false))
    (else
      (Utilities|Array|SetArrayElem (Variables|Inventory|GetContent) Slot_Index (Utilities|Struct|MakeStruct_Inventory_Slot (.item_id _output) _returnvalue (.occupied? _output) (.actor_class _output)))))
  (Class|BPIHUD|UpdatePlayerMainSlots(Message) (HUD|GetHUD (Game|GetPlayerController 0))))

(fn SpawnDroppedItems
  (bind _item_to_spawn (Variables|Helper|GetItem_To_Spawn)
    (:then
      (bind _drop_position (Class|BPIPlayer|GetDropPosition(Message) (Components|GetOwner)))
      (Game|SpawnActorfromClass _item_to_spawn (Math|Transform|MakeTransform _drop_position "0, 0, 0" "1.000000,1.000000,1.000000") "Undefined" "MultiplyWithRoot" 0 0))
    (:else)))

(fn FindItem
  (params (Item_ID_To_Find :type Name))
  (for (_array_element _array_index) (Variables|Inventory|GetContent)
    (if (== Item_ID_To_Find (.Item_ID (Utilities|Struct|BreakStruct_Inventory_Slot _array_element)))
      (return true _array_index)))
  (return false -1))

(fn AddRandomLoot
  (bind (_success_ _item_id) (CallFunction|GetRandomItemfromDB))
  (bind (_success__2 _item_id_2 _item_info) (CallFunction|GetRandomItemfromDB))
  (if (Variables|Loot|GetUnique_Loot?)
    (for _index (range (Variables|Loot|GetMin_Loot_Count) (Variables|Loot|GetMax_Loot_Count))
      (if _success__2
        (bind _output_get (LocalVariables|SetItem_To_Add _item_id_2))
        (LocalVariables|SetItem_Info _item_info)
        (bind _success__3 (Helper|FindItem _output_get))
        (if (not _success__3)
          (if (.stackable? (LocalVariables|GetItem_Info))
            (CallFunction|AddItem (LocalVariables|GetItem_To_Add) (Math|Random|RandomIntegerinRange (Variables|Loot|GetMin_Loot_Stack_Amount) (Variables|Loot|GetMax_Loot_Stack_Amount)))
            (else
              (CallFunction|AddItem (LocalVariables|GetItem_To_Add) 1))))))
    (else
      (for _index_2 (range (Variables|Loot|GetMin_Loot_Count) (Variables|Loot|GetMax_Loot_Count))
        (if _success_
          (CallFunction|AddItem _item_id (Math|Random|RandomIntegerinRange (Variables|Loot|GetMin_Loot_Stack_Amount) (Variables|Loot|GetMax_Loot_Stack_Amount))))))))