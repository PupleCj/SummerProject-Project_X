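; Base enemy character for melee combat, with health, a targetable health bar widget and a death that awards the player extra time before the actor is destroyed.
; Damage plays a hit-reaction montage chosen by damage type, while a simple state enum gates reactions and attacks.
; Attacks play indexed montages; a forward sphere trace damages the player once per call, skipping one player state.
; A Timeline-driven buffer slides the enemy forward with sweeping.
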(event Custom|ResetState)

(event Custom|OnTargeted
  (Rendering|SetVisibility (Variables|Default|GetWidget) true false))

(event Custom|AddMovement
  ;[0 0.4072 0.01161] Buffer System
)

(event Custom|Buffer
  (params (Distance :type Float%20%28single-precision%29))
  (bind _returnvalue (Transformation|GetActorLocation))
  ;[0 0.4072 0.01161] Buffer System
  (CallFunction|StopBuffer)
  (if (!= Distance 0.0)
    (bind _alpha (Timeline|Timeline PlayFromStart)
      (:Update
        (Transformation|SetActorLocation (Math|Vector|Lerp(Vector) _returnvalue (+ _returnvalue (* (Transformation|GetActorForwardVector) Distance)) _alpha) true false)))))

(event Custom|StopBuffer
  (bind _returnvalue (Transformation|GetActorLocation))
  ;[0 0.4072 0.01161] Buffer System
  (bind _alpha (Timeline|Timeline Stop)
    (:Update
      (Transformation|SetActorLocation (Math|Vector|Lerp(Vector) _returnvalue (+ _returnvalue (* (Transformation|GetActorForwardVector) (stale Custom|Buffer Distance))) _alpha) true false))))

(event Custom|EndTargeted
  (Rendering|SetVisibility (Variables|Default|GetWidget) false false))

(event Game|Damage|EventAnyDamage
  (params (Damage :type Float%20%28single-precision%29) (DamageType :type Damage%20Type%20Object%20Reference) (InstigatedBy :type Controller%20Object%20Reference) (DamageCauser :type Actor%20Object%20Reference))
  (bind _output_get (Variables|Stats|SetCurrentHealth (- (Variables|Stats|GetCurrentHealth) Damage)))
  (Default|UpdateHealth (Variables|Default|GetHealthBar))
  (if (> _output_get 0.0)
    (bind _asbp_damage_type_main (Utilities|Casting|CastToBP_DamageTypeMain DamageType))
    (if (and (Utilities|IsValid (Damage|GetHitReactionMontage (Variables|/Game/_Teale/Blueprints/HackAndSlash/DamageType/BP_DamageTypeMain.BP_DamageTypeMain_C|GetDamage%20Types _asbp_damage_type_main))) (not (State|IsCurrentStateEqualtoAny (Utilities|Array|MakeArray "NewEnumerator3"))))
      (Animation|PlayAnimMontage (Damage|GetHitReactionMontage (Variables|/Game/_Teale/Blueprints/HackAndSlash/DamageType/BP_DamageTypeMain.BP_DamageTypeMain_C|GetDamage%20Types _asbp_damage_type_main)) 1.0 "None")
      (else
        (Development|PrintString "ENEMY HIT INVALID" true true "(R=1.000000,G=0.000000,B=0.013939,A=1.000000)")))
    (else
      (Damage|PerformDeath)
      (Utilities|FlowControl|Delay (Variables|Damage|GetDeathTimer))
      (Actor|DestroyActor))))

(event EventBeginPlay
  (Utilities|FlowControl|Sequence
    (:then_0
      (Variables|Stats|SetCurrentHealth (Variables|Stats|GetMaxHealth))
      (bind _asw_enemy_health_bar (Utilities|Casting|CastToW_EnemyHealthBar (UserInterface|GetWidget (Variables|Default|GetWidget))))
      (Variables|/Game/_Barney/UI_Assets/W_EnemyHealthBar.W_EnemyHealthBar_C|SetEnemy%20Owner _asw_enemy_health_bar self)
      (Default|UpdateHealth _asw_enemy_health_bar)
      (Variables|Default|SetHealthBar _asw_enemy_health_bar))))

(fn ConstructionScript)

(fn PerformDeath
  (bind _asbp_ha_scharacter (Utilities|Casting|CastToBP_HaSCharacter (Game|GetPlayerCharacter 0)))
  (Default|AddTimeonKill _asbp_ha_scharacter 1e+01)
  (State|SetState "NewEnumerator3")
  (Animation|PlayAnimMontage (Variables|Damage|GetDeath) 1.0 "None")
  (Collision|SetCollisionEnabled (Variables|Collision|GetCapsuleComponent) "NoCollision"))

(fn GetHitReactionMontage
  (params (DamageType :type E_DamageTypes%20Enum :default "NewEnumerator0"))
  (switch Utilities|FlowControl|Switch|SwitchonE_DamageTypes DamageType
    (:NewEnumerator0
      (return 0))
    (:NewEnumerator1
      (return (Variables|HitReaction|GetHR_R)))
    (:NewEnumerator2
      (return (Variables|HitReaction|GetHR_L)))
    (:NewEnumerator3
      (return (Variables|HitReaction|GetHR_M)))
    (:NewEnumerator4
      (return (Variables|HitReaction|GetHR_Kno)))
    (:NewEnumerator5
      (return (Variables|HitReaction|GetHR_KnoOut)))))

(fn SetState
  (params (NewState :type E_States%20Enum :default "NewEnumerator0"))
  (if (Utilities|Enum|NotEqual(Enum) NewState (Variables|State|GetCurrentState))
    (Variables|State|SetCurrentState NewState)))

(fn GetState
  (return (Variables|State|GetCurrentState)))

(fn IsCurrentStateEqualtoAny
  (params (TargetArray :type Array%20of%20E_States%20Enums :default "NewEnumerator0"))
  (return (Utilities|Array|ContainsItem TargetArray (Variables|State|GetCurrentState))))

(fn CanAttack
  (bind _charactermovement (Variables|Character|GetCharacterMovement))
  (return (and (not (State|IsCurrentStateEqualtoAny (Utilities|Array|MakeArray "NewEnumerator2" "NewEnumerator1" "NewEnumerator3" "NewEnumerator4"))) (not (or (Class|NavMovementComponent|IsFlying _charactermovement) (AI|Components|NavMovement|IsFalling _charactermovement))))))

(fn PerformAttack
  (params (Index :type Integer))
  (bind _attackmontage (Variables|Default|GetAttackMontage))
  (bind _output (Utilities|Array|Get(acopy) _attackmontage Index))
  (if (CallFunction|CanAttack)
    (Utilities|IsValid _output
      (:Is%20Valid
        (State|SetState "NewEnumerator1")
        (bind _returnvalue (Animation|Montage|MontagePlay (Components|SkeletalMesh|GetAnimInstance (Variables|Character|GetMesh)) _output 1.0 "Duration" 0.0 true))
        (return _returnvalue))
      (:Is%20Not%20Valid
        (return 0.0)))
    (else
      (return 0.0))))

(fn DrawWeaponCollision
  (params (EndLocation :type Float%20%28single-precision%29) (Damage :type Float%20%28single-precision%29) (Radius :type Float%20%28single-precision%29) (DamageTypeClass :type BP%20Damage%20Type%20Main%20Class%20Reference))
  (bind _returnvalue (Transformation|GetActorLocation))
  (bind _self self)
  (Utilities|Array|Clear (Variables|Default|GetHitActors))
  (bind (_outhits _returnvalue_2) (Collision|MultiSphereTraceForObjects _returnvalue (+ (* (Transformation|GetActorForwardVector) EndLocation) _returnvalue) Radius (Utilities|Array|MakeArray "ObjectTypeQuery3") false 0 "None" true "(R=1.000000,G=0.000000,B=0.000000,A=1.000000)" "(R=0.000000,G=1.000000,B=0.000000,A=1.000000)" 2.5))
  (if _returnvalue_2
    (for _array_element _outhits
      (if (and (not (Utilities|Array|ContainsItem (Variables|Default|GetHitActors) (.HitActor (Collision|BreakHitResult _array_element)))) (Utilities|IsValid (.HitActor (Collision|BreakHitResult _array_element))))
        (bind _asbp_ha_scharacter (Utilities|Casting|CastToBP_HaSCharacter (.HitActor (Collision|BreakHitResult _array_element))))
        (if (Utilities|Enum|NotEqual(Enum) (Default|GetState _asbp_ha_scharacter) "NewEnumerator0")
          (Game|Damage|ApplyDamage (.HitActor (Collision|BreakHitResult _array_element)) Damage (Pawn|GetController _self) _self DamageTypeClass)
          (Utilities|Array|AddUnique (Variables|Default|GetHitActors) (.HitActor (Collision|BreakHitResult _array_element))))))))