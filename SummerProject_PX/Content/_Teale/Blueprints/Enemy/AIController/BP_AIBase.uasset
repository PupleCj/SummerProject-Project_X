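; Base AI controller for enemies that starts each enemy's behaviour tree on possession.
; It only proceeds for BP_Base_Enemy pawns, running the tree stored on that enemy.
; It then writes the first player character as the target and a strafe distance into the blackboard, and sets focus on the player.
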(event EventPossess
  (params (PossessedPawn :type Pawn%20Object%20Reference))
  (bind _asbp_base_enemy (Utilities|Casting|CastToBP_Base_Enemy PossessedPawn))
  (AI|RunBehaviorTree self (Variables|/Game/_Teale/Blueprints/Enemy/BP_Base_Enemy.BP_Base_Enemy_C|GetBehaviourTree _asbp_base_enemy))
  (CallFunction|SetBlackboardKeys)
  (AI|SetFocus (Game|GetPlayerCharacter 0)))

(fn ConstructionScript)

(fn SetBlackboardKeys
  (bind _self self)
  (bind _returnvalue (AI|GetBlackboard _self))
  (Utilities|IsValid _returnvalue
    (:Is%20Valid
      (AI|Components|Blackboard|SetValueasObject _returnvalue (Variables|Default|GetTargetKeyName) (Game|GetPlayerCharacter 0))
      (AI|Components|Blackboard|SetValueasFloat _returnvalue (Variables|Default|GetStrafeDistanceKeyName) (Variables|Default|GetStrafeDistance)))))