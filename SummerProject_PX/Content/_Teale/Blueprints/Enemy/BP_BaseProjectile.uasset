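; Base enemy projectile that damages the player character when its Box collision overlaps them.
; A hit applies the Damage value, spawns an explosion particle and destroys the projectile, but is ignored while the character has i-frames or is in one excluded state.
; Overlapping an actor whose class is exactly StaticMeshActor spawns a fireball particle at that actor's location and destroys the projectile.
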(event OnComponentBeginOverlap(Box)
  (params (OverlappedComponent :type Primitive%20Component%20Object%20Reference) (OtherActor :type Actor%20Object%20Reference) (OtherComp :type Primitive%20Component%20Object%20Reference) (OtherBodyIndex :type Integer) (bFromSweep :type Boolean) (SweepResult :type Hit%20Result%20Structure%20%28by%20ref%29))
  (bind _asbp_ha_scharacter (Utilities|Casting|CastToBP_HaSCharacter OtherActor)
    (:then
      (if (and (not (Default|IsIFramesEnabled _asbp_ha_scharacter)) (Utilities|Enum|NotEqual(Enum) (Default|GetState _asbp_ha_scharacter) "NewEnumerator3"))
        (Game|Damage|ApplyDamage _asbp_ha_scharacter (Variables|Default|GetDamage) 0 0 "/Game/_Teale/Blueprints/HackAndSlash/DamageType/DT_Middle.DT_Middle_C")
        (Effects|SpawnEmitteratLocation "/Game/StarterContent/Particles/P_Explosion.P_Explosion" (Transformation|GetActorLocation OtherActor))
        (Actor|DestroyActor)))
    (:CastFailed
      (if (== (Utilities|GetClass OtherActor) "/Script/Engine.StaticMeshActor")
        (Effects|SpawnEmitteratLocation "/Game/_Teale/Assets/FXVarietyPack/Particles/P_ky_fireBall.P_ky_fireBall" (Transformation|GetActorLocation OtherActor))
        (Actor|DestroyActor)))))

(fn ConstructionScript)